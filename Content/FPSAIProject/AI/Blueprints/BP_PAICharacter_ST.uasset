(event OnHealthChanged(HealthComponent)
  (params (Instigator :type Actor%20Object%20Reference) (OwningComp :type P%20Health%20Component%20Object%20Reference) (NewHealth :type Float%20%28single-precision%29) (Delta :type Float%20%28single-precision%29))
  (bind _as_bp_paicharacter_st (Variables|Default|GetAs%20BP%20PAICharacter%20ST))
  (bind _as_bp_paicharacter_st_2 (Variables|Default|GetAs%20BP%20PAICharacter%20ST))
  (Variables|Default|SetIsPlayerVisible true)
  (if (GameplayTags|HasTag (Variables|Default|GetGameplayTagContainer) "(TagName=\"Enemy.Type.Zombie.Crawl\")" true)
    (bind _animmontage (CallFunction|GetAnimationMontages _as_bp_paicharacter_st_2 _as_bp_paicharacter_st_2 "NewEnumerator6"))
    (Animation|PlayAnimMontage (Variables|Default|GetAs%20BP%20PAICharacter%20ST) _animmontage 1.0 "None")
    (else
      (bind _animmontage_2 (CallFunction|GetAnimationMontages _as_bp_paicharacter_st _as_bp_paicharacter_st "NewEnumerator0"))
      (Animation|PlayAnimMontage (Variables|Default|GetAs%20BP%20PAICharacter%20ST) _animmontage_2 1.0 "None"))))

(event Custom|AssignPlayerDistance
  (params (QueryInstance :type Env%20Query%20Instance%20Blueprint%20Wrapper%20Object%20Reference) (QueryStatus :type EEnvQueryStatus%20Enum :default "Processing"))
  (bind _resultlocations (AI|EQS|GetQueryResultsasLocations QueryInstance))
  (if (Utilities|Array|IsValidIndex _resultlocations)
    (Variables|Default|SetLocationToPlayer _resultlocations)
    (EventDispatchers|UnbindallEventsfromOnQueryFinishedEvent (stale EventTick _returnvalue))))

(event Custom|AssignPlayer
  (params (QueryInstance :type Env%20Query%20Instance%20Blueprint%20Wrapper%20Object%20Reference) (QueryStatus :type EEnvQueryStatus%20Enum :default "Processing"))
  (bind _resultlocations (AI|EQS|GetQueryResultsasLocations QueryInstance))
  (if (Utilities|Array|IsValidIndex _resultlocations)
    (Variables|Default|SetLocationToPlayer _resultlocations)
    (EventDispatchers|UnbindallEventsfromOnQueryFinishedEvent (stale EventTick _returnvalue_2))))

(event EventBeginPlay
  (bind _returnvalue (Pawn|GetController))
  (bind _returnvalue_2 (Pawn|GetControlledPawn _returnvalue))
  (Variables|Default|SetIsAlive (> (Variables|/Script/FPSAIProj.PHealthComponent|GetHealth (Variables|Default|GetHealthComponent)) 0.0))
  (Utilities|IsValid _returnvalue_2
    (:Is%20Valid
      (bind _asbp_paicharacter_st (Utilities|Casting|CastToBP_PAICharacter_ST _returnvalue_2))
      (Variables|BP_PAICharacter_ST_C|SetAs%20BP%20PAICharacter%20ST _asbp_paicharacter_st _asbp_paicharacter_st))
    (:Is%20Not%20Valid
      (Development|PrintString "Incorrect Controller"))))

(event EventTick
  (params (DeltaSeconds :type Float%20%28single-precision%29))
  (if (Variables|Default|GetIsPlayerVisible)
    (Transformation|SetActorRotation (Variables|Default|GetAs%20BP%20PAICharacter%20ST) (Math|Rotator|FindLookatRotation (Transformation|GetActorLocation (Variables|Default|GetAs%20BP%20PAICharacter%20ST)) (Transformation|GetActorLocation (Game|Player|GetPlayerPawn 0)))))
  (CallFunction|CreateHealthBar)
  (if (== (Variables|Default|GetEnemyType) "(TagName=\"Enemy.Type.Skeleton.Bow\")")
    (bind _returnvalue (AI|EQS|RunEQSQuery "/Game/FPSAIProject/AI/EQS/Query_FindNearLocationDistanceEnemy.Query_FindNearLocationDistanceEnemy" (Game|Player|GetPlayerPawn 0) "AllMatching"))
    (EventDispatchers|BindEventtoOnQueryFinishedEvent _returnvalue (delegate Custom|AssignPlayerDistance))
    (else
      (bind _returnvalue_2 (AI|EQS|RunEQSQuery "/Game/FPSAIProject/AI/EQS/Query_FindNearLocation.Query_FindNearLocation" (Game|Player|GetPlayerPawn 0) "AllMatching"))
      (EventDispatchers|BindEventtoOnQueryFinishedEvent _returnvalue_2 (delegate Custom|AssignPlayer)))))

(fn ConstructionScript)

(fn HitDetect
  (params (AIPawn :type BP%20PAI%20Character%20ST%20Object%20Reference))
  (bind _bonename (CallFunction|GetAnimationMontages AIPawn AIPawn "NewEnumerator0"))
  (bind _outhit (Collision|SphereTraceForObjects (Transformation|GetSocketLocation (Variables|/Script/Engine.Character|GetMesh AIPawn) _bonename) (Transformation|GetSocketLocation (Variables|/Script/Engine.Character|GetMesh AIPawn) _bonename) 1.5e+02 (Utilities|Array|MakeArray "ObjectTypeQuery3") false 0 "ForDuration"))
  (bind _asbp_first_person_character (Utilities|Casting|CastToBP_FirstPersonCharacter (.HitActor (Collision|BreakHitResult _outhit))))
  (Class|PHealthComponent|ApplyHealthChange (Variables|/Script/FPSAIProj.FPSAIProjCharacter|GetHealthComponent _asbp_first_person_character) _asbp_first_person_character -2.0))

(fn GetAnimationMontages
  (params (AIPawn :type BP%20PAI%20Character%20ST%20Object%20Reference%20%28by%20ref%29) (AnimationType :type E_ActionType%20Enum%20%28by%20ref%29 :default "NewEnumerator0"))
  (bind _animationarray (Variables|Default|GetAnimationArray))
  (bind _outitem (Utilities|Array|Random _animationarray))
  (bind (_charactertype _animmontage _bonename _actiontype) (Utilities|Struct|BreakSAnimationMontages _outitem))
  (Utilities|Array|Clear (Variables|Default|GetAnimationArray))
  (bind _outrownames (DataTable|GetDataTableRowNames "/Game/FPSAIProject/AI/AnimationMontages_DT.AnimationMontages_DT"))
  (bind _array_element (Utilities|Array|ForEachLoopwithBreak _outrownames)
    (:LoopBody
      (bind _returnvalue (Utilities|GetDataTableRow "/Game/FPSAIProject/AI/AnimationMontages_DT.AnimationMontages_DT" _array_element)
        (:then
          (if (and (Utilities|Enum|Equal(Enum) (Utilities|String|EnumtoString (.CharacterType (Utilities|Struct|BreakSAnimationMontages _returnvalue))) (Utilities|String|EnumtoString (Variables|BP_PAICharacter_ST_C|GetCharacterType AIPawn))) (Utilities|Enum|Equal(Enum) (Utilities|String|EnumtoString (.ActionType (Utilities|Struct|BreakSAnimationMontages _returnvalue))) (Utilities|String|EnumtoString AnimationType)))
            (Utilities|Array|Add (Variables|Default|GetAnimationArray) _returnvalue)))))
    (:Completed
      (if (Utilities|Array|IsNotEmpty (Variables|Default|GetAnimationArray))
        (return _charactertype _animmontage _bonename _actiontype)))))

(fn GetPawnLocation
  (return (Transformation|GetActorLocation)))

(fn HandleSightSense
  (params (Actor :type Actor%20Object%20Reference%20%28by%20ref%29) (Stimulus :type AI%20Stimulus%20Structure))
  (bind _returnvalue (Class|AIPerceptionSystem|GetSenseClassforStimulus Stimulus))
  (if (== _returnvalue "/Script/AIModule.AISense_Sight")
    (if (== Actor (Game|GetPlayerCharacter 0))
      (Variables|Default|SetIsPlayerVisible true)
      (else
        (return)))
    (else
      (return))))

(fn HandleSoundSense
  (params (Stimulus :type AI%20Stimulus%20Structure%20%28by%20ref%29) (Actor :type Actor%20Object%20Reference))
  (bind _returnvalue (Class|AIPerceptionSystem|GetSenseClassforStimulus Stimulus))
  (if (== _returnvalue "/Script/AIModule.AISense_Hearing")
    (if (== Actor (Game|GetPlayerCharacter 0))
      (Variables|Default|SetIsPlayerVisible true)
      (else
        (return)))
    (else
      (return))))

(fn CreateHealthBar
  (bind _healthcomponent (Variables|Default|GetHealthComponent))
  (bind _health (Variables|/Script/FPSAIProj.PHealthComponent|GetHealth _healthcomponent))
  (bind _asenemy_health_bar (Utilities|Casting|CastToEnemy_HealthBar (UserInterface|GetWidget (Variables|Default|GetHealthBar))))
  (Variables|Default|SetEnemyHealth _health)
  (Progress|SetPercent (Variables|/Game/FPSAIProject/UI/Enemy_HealthBar.Enemy_HealthBar_C|GetProgressBar _asenemy_health_bar) (/ _health (Variables|/Script/FPSAIProj.PHealthComponent|GetHealthMax _healthcomponent)))
  (Transformation|SetWorldRotation (Variables|Default|GetHealthBar) (Math|Rotator|FindLookatRotation (Transformation|GetWorldLocation (Variables|Default|GetHealthBar)) (Transformation|GetWorldLocation (Variables|/Script/Engine.PlayerCameraManager|GetTransformComponent (Game|GetPlayerCameraManager 0)))) false false)
  (return))

(fn ReserveAttackToken
  (params (Amount :type Integer)))