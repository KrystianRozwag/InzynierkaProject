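; BP_HealthPotion is a pickup that heals the first-person player character when it enters the potion's box.
; On overlap, it acts only if that character's HealthComponent reads Health below a hardcoded 100.
; It then applies the gap to HealthMax, clamped between zero and 100, through ApplyHealthChange and destroys itself, so the potion stays in place otherwise.
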(event OnComponentBeginOverlap(Box)
  (params (OverlappedComponent :type Primitive%20Component%20Object%20Reference) (OtherActor :type Actor%20Object%20Reference) (OtherComp :type Primitive%20Component%20Object%20Reference) (OtherBodyIndex :type Integer) (bFromSweep :type Boolean) (SweepResult :type Hit%20Result%20Structure%20%28by%20ref%29))
  (bind _asbp_first_person_character (Utilities|Casting|CastToBP_FirstPersonCharacter OtherActor))
  (Utilities|IsValid _asbp_first_person_character
    (:Is%20Valid
      (if (< (Variables|/Script/FPSAIProj.PHealthComponent|GetHealth (Variables|/Script/FPSAIProj.FPSAIProjCharacter|GetHealthComponent _asbp_first_person_character)) 1e+02)
        (Class|PHealthComponent|ApplyHealthChange (Variables|/Script/FPSAIProj.FPSAIProjCharacter|GetHealthComponent _asbp_first_person_character) 0 (Math|Float|Clamp(Float) (- (Variables|/Script/FPSAIProj.PHealthComponent|GetHealthMax (Variables|/Script/FPSAIProj.FPSAIProjCharacter|GetHealthComponent _asbp_first_person_character)) (Variables|/Script/FPSAIProj.PHealthComponent|GetHealth (Variables|/Script/FPSAIProj.FPSAIProjCharacter|GetHealthComponent _asbp_first_person_character))) 0.0 1e+02))
        (Actor|DestroyActor)))))

(fn ConstructionScript)